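; Base enemy Blueprint that handles the sound and visual feedback when an enemy is defeated.
; On BeginPlay it binds to the Defeated event, which plays a defeat cue at the enemy's location and destroys the actor.
; The Destroyed event spawns BP_EnemyDestroyedVFX at its location and rotation, so the effect follows any destruction, not only defeat.
; A TurnCharacter function flips the actor by combining its rotation with a half turn.
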(event `self.ReceiveBeginPlay`
  (`parent.ReceiveBeginPlay`)
  (add `self.Defeated` (delegate `OnDefeated`)))

(event `OnDefeated`
  (`GameplayStatics.PlaySoundAtLocation` "/Game/Audio/SFX/Enemy_Defeat_Cue.Enemy_Defeat_Cue" (`self.K2_GetActorLocation`) (struct) 1.0 1.0 0.0 null null null null)
  (`self.K2_DestroyActor`))

(event `self.ReceiveDestroyed`
  (`|SpawnActorFromClass` "/Game/Blueprints/VFX/BP_EnemyDestroyedVFX.BP_EnemyDestroyedVFX_C" (`KismetMathLibrary.MakeTransform` (`self.K2_GetActorLocation`) (`self.K2_GetActorRotation`)) "Undefined" "MultiplyWithRoot" null null))

(fn `TurnCharacter`
  (`self.K2_SetActorRotation` (`KismetMathLibrary.ComposeRotators` (`self.K2_GetActorRotation`) (struct :`Yaw` 180.0))))

(fn `UserConstructionScript`
  (`parent.UserConstructionScript`))