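; BP_BatEnemy is a bat enemy that moves endlessly back and forth between two marker points.
; BeginPlay caches the TopPos and BottomPos world locations, sets the MoveAnim timeline's play rate from MovePlayRate and starts moving.
; The timeline's Alpha lerps the actor location between the cached points without sweeping.
; Each time the timeline finishes, a FlipFlop alternates between reversing it and playing it from the start.
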(event `self.ReceiveBeginPlay`
  (`parent.ReceiveBeginPlay`)
  (set `self.WorldTopPos` (`SceneComponent.K2_GetComponentLocation` (`self.TopPos`)))
  (set `self.WorldBottomPos` (`SceneComponent.K2_GetComponentLocation` (`self.BottomPos`)))
  (`TimelineComponent.SetPlayRate` (`self.MoveAnim`) (`self.MovePlayRate`))
  (`self.MoveFoward`))

(event `MoveFoward`
  (bind (_direction _alpha) (`Timeline|MoveAnim` :!via `PlayFromStart` :!label _label)
    (:`Update`
      (`self.K2_SetActorLocation` (`KismetMathLibrary.VLerp` (`self.WorldTopPos`) (`self.WorldBottomPos`) _alpha)))
    (:`Finished`
      (`/Engine/EditorBlueprintResources/StandardMacros.FlipFlop`
        (:`A`
          (`self.MoveBackward`))
        (:`B`
          (`self.MoveFoward`))))))

(event `MoveBackward`
  (goto _label :!via `ReverseFromEnd`))

(fn `UserConstructionScript`
  (`parent.UserConstructionScript`))