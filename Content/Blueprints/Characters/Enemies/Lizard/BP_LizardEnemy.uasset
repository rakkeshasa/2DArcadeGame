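; BP_LizardEnemy is a lizard enemy that shoots fireball projectiles.
; ShootFireball only plays the Shoot animation as an override on the animation component's instance.
; A separate SpawnProjectile function spawns BP_EnemyLizardProjectile at the ShootPos transform and plays the shot sound at the actor's location.
; Neither function is called within this Blueprint, and its event graph holds only disabled default events.
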(fn `ShootFireball`
  (`PaperZDAnimInstance.K2_PlayAnimationOverride` (`PaperZDAnimationComponent.AnimInstance` (`self.AnimationComponent`)) "/Game/Blueprints/Characters/Enemies/Lizard/AnimSequences/Shoot.Shoot" "DefaultSlot" 1.0 0.0))

(fn `SpawnProjectile`
  (bind _shootpos (`self.ShootPos`))
  (`|SpawnActorFromClass` "/Game/Blueprints/Projectile/Enemy/BP_EnemyLizardProjectile.BP_EnemyLizardProjectile_C" (`KismetMathLibrary.MakeTransform` (`SceneComponent.K2_GetComponentLocation` _shootpos) (`SceneComponent.K2_GetComponentRotation` _shootpos)) "AlwaysSpawn" "MultiplyWithRoot" null null)
  (`GameplayStatics.PlaySoundAtLocation` "/Game/Audio/SFX/Shoot_Lizard_Cue.Shoot_Lizard_Cue" (`self.K2_GetActorLocation`) (struct) 1.0 1.0 0.0 null null null null))

(fn `UserConstructionScript`
  (`parent.UserConstructionScript`))